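; BP_HighscoreSave holds the high score list, presumably for saving, and keeps only the top four entries.
; AddHighScore appends a new entry, calls SortSaveData, then trims the list.
; SortSaveData orders scores highest first with a selection sort, repeatedly moving the result of DetermineHighestScoreValue into a temporary list.
; DetermineLowestScoreValue returns the lowest entry and its index but is not called within this Blueprint.
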(fn `AddHighScore`
  (params (NewScore :type "/Game/Blueprints/BP_HighScoreStruct Structure"))
  (bind _savestructlist (`self.SaveStructList`))
  (`KismetArrayLibrary.Array_Add` _savestructlist NewScore)
  (`self.SortSaveData`)
  (`KismetArrayLibrary.Array_Resize` (`self.SaveStructList`) (`KismetMathLibrary.Min` 4 (`KismetArrayLibrary.Array_Length` _savestructlist))))

(fn `DetermineHighestScoreValue`
  (returns (HighestScoreStruct :type "/Game/Blueprints/BP_HighScoreStruct Structure") (HighestScoreIndex :type Integer))
  (locals (HighestScore :type "Float (double-precision)") (HighestIndex :type Integer))
  (bind _highestindex (`local.HighestIndex`))
  (for (_array_element _array_index) (`self.SaveStructList`)
    (if (== _array_index 0)
      (set `local.HighestScore` (`.Score_5_6622C55442435A271E615CB49A861E8D` (break `/Game/Blueprints/BP_HighScoreStruct` _array_element)) :!label _label)
      (set `local.HighestIndex` _array_index)
      (elif (> (`.Score_5_6622C55442435A271E615CB49A861E8D` (break `/Game/Blueprints/BP_HighScoreStruct` _array_element)) (`local.HighestScore`))
        (goto _label))))
  (return (`|GetArrayItem` (`self.SaveStructList`) _highestindex) _highestindex))

(fn `DetermineLowestScoreValue`
  (returns (LowestScoreStruct :type "/Game/Blueprints/BP_HighScoreStruct Structure") (LowestScoreIndex :type Integer))
  (locals (LowestScore :type "Float (double-precision)") (LowestIndex :type Integer))
  (bind _lowestindex (`local.LowestIndex`))
  (for (_array_element _array_index) (`self.SaveStructList`)
    (if (== _array_index 0)
      (set `local.LowestScore` (`.Score_5_6622C55442435A271E615CB49A861E8D` (break `/Game/Blueprints/BP_HighScoreStruct` _array_element)) :!label _label)
      (set `local.LowestIndex` _array_index)
      (elif (< (`.Score_5_6622C55442435A271E615CB49A861E8D` (break `/Game/Blueprints/BP_HighScoreStruct` _array_element)) (`local.LowestScore`))
        (goto _label))))
  (return (`|GetArrayItem` (`self.SaveStructList`) _lowestindex) _lowestindex))

(fn `SortSaveData`
  (locals (TempSaveStructList :type "Array of /Game/Blueprints/BP_HighScoreStruct Structure"))
  (while (> (`KismetArrayLibrary.Array_Length` (`self.SaveStructList`)) 0)
    (bind (_highestscorestruct _highestscoreindex) (`self.DetermineHighestScoreValue`))
    (`KismetArrayLibrary.Array_Add` (`local.TempSaveStructList`) _highestscorestruct)
    (`KismetArrayLibrary.Array_Remove` (`self.SaveStructList`) _highestscoreindex))
  (set `self.SaveStructList` (`local.TempSaveStructList`)))