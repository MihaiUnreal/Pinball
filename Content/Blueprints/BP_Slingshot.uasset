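; Pinball-style slingshot bumper that kicks an overlapping BP_Ball away and adds score through BP_GameMode.
; On overlap it applies an impulse to the ball opposite the capsule's forward vector and plays the SlingBounce timeline.
; The timeline animates the band by driving PercentOut on a dynamic material created in the construction script.
; A DoOnce, reset on end overlap, limits the hit sound to once per overlap.
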(event `self.ReceiveActorBeginOverlap`
  (params (OtherActor :type "Actor Object Reference"))
  (bind _asbp_ball (cast `/Game/Blueprints/BP_Ball` OtherActor))
  (bind _asbp_game_mode (cast `/Game/Blueprints/BP_GameMode` (`GameplayStatics.GetGameMode`)))
  (`/Game/Blueprints/BP_GameMode.AddScore` _asbp_game_mode 20.0) ; add 20 points
  (`PrimitiveComponent.AddImpulse` (`/Game/Blueprints/BP_Ball.Ball` _asbp_ball) (* (`SceneComponent.GetForwardVector` (`self.Capsule`)) -2500.0) "None" false)
  (bind (_direction _bounce) (`Timeline|SlingBounce` :!via `PlayFromStart`)
    (:`Update`
      (bind _asmaterial_instance_dynamic (cast `MaterialInstanceDynamic` (`PrimitiveComponent.GetMaterial` (`self.MorphSlingband`) 2)))
      (`MaterialInstanceDynamic.SetScalarParameterValue` _asmaterial_instance_dynamic "PercentOut" _bounce)
      (`/Engine/EditorBlueprintResources/StandardMacros.DoOnce` false :!label _label ; via DoOnce node we ensure the sound is play only once on overlap!
        (:`Completed`
          (`GameplayStatics.SpawnSoundAttached` "/Game/Sounds/SlingshotHit.SlingshotHit" (`self.MorphSlingband`) "None" (0.0 0.0 0.0) (struct) "KeepRelativeOffset" false 1.0 1.0 0.0 null null))))))

(event `self.ReceiveActorEndOverlap`
  (params (OtherActor :type "Actor Object Reference"))
  (`self.ResetPlaySound`))

(event `ResetPlaySound`
  (goto _label :!via `Reset`))

(fn `UserConstructionScript`
  (`PrimitiveComponent.CreateDynamicMaterialInstance` (`self.MorphSlingband`) 2 null "None") ; Band is index 2
)