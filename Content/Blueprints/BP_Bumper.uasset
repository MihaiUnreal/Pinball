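; Pinball-style bumper actor that knocks the ball away and awards points on overlap.
; Overlap with BP_Ball calls Bump, which applies a mass-independent impulse away from the bumper, spawns sparks and sound, and adds score through BP_GameMode.
; A timeline then drives the mechanism's vertical offset, light intensity and emissive boost on a dynamic material created in the construction script.
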(event `self.ReceiveActorBeginOverlap`
  (params (OtherActor :type "Actor Object Reference"))
  (bind _asbp_ball (cast `/Game/Blueprints/BP_Ball` OtherActor))
  (`self.Bump` _asbp_ball))

(event `Bump`
  (params (Ball :type "/Game/Blueprints/BP_Ball Object Reference"))
  (`PrimitiveComponent.AddImpulse` (`/Game/Blueprints/BP_Ball.Ball` Ball) (* (`KismetMathLibrary.GetDirectionUnitVector` (`self.K2_GetActorLocation`) (`self.K2_GetActorLocation` Ball)) 2500.0) "None" true)
  (`GameplayStatics.SpawnEmitterAtLocation` "/Game/Blueprints/PS_BumperSparks.PS_BumperSparks" (`SceneComponent.K2_GetComponentLocation` (`self.BumperMechanism`)))
  (`GameplayStatics.SpawnSoundAttached` "/Game/Sounds/BumperHit.BumperHit" (`self.BumperBase`) "None" (0.0 0.0 0.0) (struct) "KeepRelativeOffset" false 1.0 1.0 0.0 null null)
  (bind _asbp_game_mode (cast `/Game/Blueprints/BP_GameMode` (`GameplayStatics.GetGameMode`))
    (:`then`
      (`/Game/Blueprints/BP_GameMode.AddScore` _asbp_game_mode 10.0) ; add 10 points
      (bind (_direction _bumalpha) (`Timeline|BumpTimeline` :!label _label)
        (:`Update`
          (`SceneComponent.K2_SetRelativeLocation` (`self.BumperMechanism`) (`KismetMathLibrary.VLerp` (0.0 0.0 0.0) (0.0 0.0 -70.0) _bumalpha) false false)
          (`LightComponent.SetIntensity` (`self.Light`) (`KismetMathLibrary.Lerp` 0.0 5000.0 _bumalpha))
          (`MaterialInstanceDynamic.SetScalarParameterValue` (`self.BumperTopMID`) "EmissiveBoost" (`KismetMathLibrary.Lerp` 0.0 30.0 _bumalpha)))))
    (:`CastFailed`
      (goto _label))))

(fn `UserConstructionScript`
  (bind _returnvalue (`PrimitiveComponent.CreateDynamicMaterialInstance` (`self.BumperBase`) 1 null "None"))
  (set `self.BumperTopMID` _returnvalue))