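; BP_ForceMovementZone is a zone that redirects a BP_Ball along its Arrow component's forward axis when the ball begins overlapping it.
; It converts the ball's velocity to Arrow-local space and interpolates toward a target with clamped positive X and zero Y and Z.
; The result returns to world space and replaces the ball's physics velocity in one InterpSpeed-scaled step per overlap, with no per-tick update.
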(event `self.ReceiveActorBeginOverlap`
  (params (OtherActor :type "Actor Object Reference"))
  (bind _returnvalue (`KismetMathLibrary.InverseTransformDirection` (`SceneComponent.K2_GetComponentToWorld` (`self.Arrow`)) (`self.GetVelocity` OtherActor)))
  (bind _asbp_ball (cast `/Game/Blueprints/BP_Ball` OtherActor))
  (`PrimitiveComponent.SetPhysicsLinearVelocity` (`/Game/Blueprints/BP_Ball.Ball` _asbp_ball) (`KismetMathLibrary.TransformDirection` (`SceneComponent.K2_GetComponentToWorld` (`self.Arrow`)) (`KismetMathLibrary.VInterpTo` _returnvalue (`KismetMathLibrary.MakeVector` (`KismetMathLibrary.FClamp` (.x _returnvalue) 800.0 20000.0)) (`GameplayStatics.GetWorldDeltaSeconds`) (`self.Interp Speed`))) false "None"))

(event `self.ReceiveActorEndOverlap`
  (params (OtherActor :type "Actor Object Reference"))
  (cast `/Game/Blueprints/BP_Ball` OtherActor))

(fn `UserConstructionScript`)